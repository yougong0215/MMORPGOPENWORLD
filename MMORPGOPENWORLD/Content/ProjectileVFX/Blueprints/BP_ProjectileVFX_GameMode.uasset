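; Demo game mode for the ProjectileVFX pack that previews Niagara projectile effects in game.
; Right click cycles through an array of effects and prints the current ID and name.
; Left click spawns the selected effect at the deprojected cursor position, offset forward and right, facing along the controller rotation.
; For the Thunder effect, a forward line trace sets the beam end parameter to the hit distance, capped at a maximum range.
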(event `self.ReceiveBeginPlay`
  (bind _returnvalue (`GameplayStatics.GetPlayerController` 0))
  ;[1 1 1] Sample function - Fix Mouse Location for Niagara display in this product
  (`self.EnableInput` _returnvalue)
  (set `PlayerController.bShowMouseCursor` false _returnvalue)
  (bind _output_get (set `self.Niagara ID` 0))
  (set `self.Niagara Ref` (`|GetArrayItem` (`self.Niagara Matrix`) _output_get))
  (`KismetSystemLibrary.PrintString` (`KismetStringLibrary.Concat_StrStr` "Niagara ID: " (`KismetStringLibrary.Conv_IntToString` (`self.Niagara ID`)) "    NIagara Name:" (`KismetSystemLibrary.GetDisplayName` (`self.Niagara Ref`)))))

(event `Key|LeftMouseButton`
  (params (Key :type "Key Structure"))
  (bind _returnvalue (`GameplayStatics.GetPlayerController` 0))
  (bind _returnvalue_2 (`self.K2_GetActorRotation` _returnvalue))
  (bind (_worldlocation _worlddirection) (`PlayerController.DeprojectMousePositionToWorld` _returnvalue))
  ;[1 1 1] Sample function - Create Niagara on game screen
  (:`Pressed`
    (bind _returnvalue_3 (`NiagaraFunctionLibrary.SpawnSystemAtLocation` (`self.Niagara Ref`) (+ _worldlocation (+ _worlddirection (* (`KismetMathLibrary.GetForwardVector` _returnvalue_2) 400.0) (* (`KismetMathLibrary.GetRightVector` _returnvalue_2) 200.0))) _returnvalue_2))
    ;;[1 0.2123 0.27] User Parameter setting for "Beam End Position" in VFX_Thunder
    (if (== (`FXSystemComponent.GetFXSystemAsset` _returnvalue_3) "/Game/ProjectileVFX/Niagara/NS_VFX_Thunder.NS_VFX_Thunder")
      (bind _returnvalue_4 (`SceneComponent.K2_GetComponentLocation` _returnvalue_3))
      (bind (_outhit _returnvalue_5) (`KismetSystemLibrary.LineTraceSingle` _returnvalue_4 (+ _returnvalue_4 (* (`KismetMathLibrary.GetForwardVector` (`SceneComponent.K2_GetComponentRotation` _returnvalue_3)) 7000.0)) "TraceTypeQuery1"))
      (if _returnvalue_5
        (bind (_bblockinghit _binitialoverlap _time _distance) (`GameplayStatics.BreakHitResult` _outhit))
        (if (>= _distance 7000.0)
          (`FXSystemComponent.SetVectorParameter` _returnvalue_3 "Beam End Position" (7000.0 0.0 0.0) :!label _label)
          (else
            (`FXSystemComponent.SetVectorParameter` _returnvalue_3 "Beam End Position" (`KismetMathLibrary.MakeVector` _distance))))
        (else
          (goto _label))))))

(event `Key|RightMouseButton`
  (params (Key :type "Key Structure"))
  ;[1 1 1] Sample function - Create Niagara on game screen
  (:`Pressed`
    (if (>= (`self.Niagara ID`) 14)
      (bind _output_get (set `self.Niagara ID` 0))
      (set `self.Niagara Ref` (`|GetArrayItem` (`self.Niagara Matrix`) _output_get))
      (else
        (bind _output_get_2 (set `self.Niagara ID` (+ (`self.Niagara ID`) 1)))
        (set `self.Niagara Ref` (`|GetArrayItem` (`self.Niagara Matrix`) _output_get_2))))
    (`KismetSystemLibrary.PrintString` (`KismetStringLibrary.Concat_StrStr` "Niagara ID: " (`KismetStringLibrary.Conv_IntToString` (`self.Niagara ID`)) "    NIagara Name:" (`KismetSystemLibrary.GetDisplayName` (`self.Niagara Ref`))))))

(fn `UserConstructionScript`)